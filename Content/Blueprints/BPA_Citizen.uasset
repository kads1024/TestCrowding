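; Citizen actor that loops through a list of Points using boids-style steering, tuned by a settings set passed to Initialize.
; Each tick adds target-seeking force, plus avoidance when a forward sphere trace hits a Pawn, to a speed-clamped velocity.
; Avoidance takes the first clear direction from golden-ratio sphere directions precomputed at BeginPlay.
; Movement is per frame, unscaled by delta time, and rotation faces the target.
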(event `self.ReceiveBeginPlay`
  (set `self.TransformCache` (`self.GetTransform`))
  (set `self.RDirs` (`self.CollisionHelper`))
  (set `self.CachedForward` (`self.GetActorForwardVector`)))

(event `self.ReceiveTick`
  (params (DeltaSeconds :type "Float (single-precision)"))
  (`self.UpdateCitizen` DeltaSeconds)
  (if (<= (`KismetMathLibrary.VSize` (- (`self.Position`) (`self.K2_GetActorLocation` (`self.Target`)))) 300.0)
    (bind _result (`/Engine/EditorBlueprintResources/StandardMacros.IncrementInt` (`self.CurrentTargetIndex`))
      (:`  `
        (set `self.CurrentTargetIndex` (mod _result (`KismetArrayLibrary.Array_Length` (`self.Points`))))
        (set `self.Target` (`|GetArrayItem` (`self.Points`) (`self.CurrentTargetIndex`)))))))

(fn `CollisionHelper`
  (returns (OutDir :type "Array of Vector Structure"))
  (locals (NumDirections :type Integer :default 300) (Directions :type "Array of Vector Structure") (GoldenRatio :type "Float (double-precision)") (AngleIncrement :type "Float (double-precision)") (t :type "Float (double-precision)") (inclination :type "Float (double-precision)") (azimuth :type "Float (double-precision)") (x :type "Float (double-precision)") (y :type "Float (double-precision)") (z :type "Float (double-precision)"))
  (`KismetArrayLibrary.Array_Resize` (`local.Directions`) (`local.NumDirections`))
  (bind _output_get (set `local.GoldenRatio` (/ (+ (`KismetMathLibrary.Sqrt` 5.0) 1.0) 2.0)))
  (set `local.AngleIncrement` (* _output_get (`KismetMathLibrary.GetPI`) 2.0))
  (for _index (range 1 (+ (`local.NumDirections`) 1))
    (bind _returnvalue (- _index 1))
    (bind _output_get_2 (set `local.t` (/ (`KismetMathLibrary.Conv_IntToDouble` _returnvalue) (`KismetMathLibrary.Conv_IntToDouble` (`local.NumDirections`)))))
    (set `local.inclination` (`KismetMathLibrary.Acos` (- 1.0 (* _output_get_2 2.0))))
    (set `local.azimuth` (* (`local.AngleIncrement`) (- _index 1)))
    (set `local.x` (* (`KismetMathLibrary.Sin` (`local.inclination`)) (`KismetMathLibrary.Cos` (`local.azimuth`))))
    (set `local.y` (* (`KismetMathLibrary.Sin` (`local.inclination`)) (`KismetMathLibrary.Sin` (`local.azimuth`))))
    (set `local.z` (`KismetMathLibrary.Cos` (`local.inclination`)))
    (`KismetArrayLibrary.Array_Set` (`local.Directions`) _returnvalue (`KismetMathLibrary.MakeVector` (`local.z`) (`local.x`) (`local.y`))))
  (return (`local.Directions`)))

(fn `Initialize`
  (params (InCitSet :type "/Game/Blueprints/S_CitizenSetting Structure"))
  (locals (StartSpeed :type "Float (double-precision)"))
  (bind (_citizenset_minspeed _citizenset_maxspeed) (break `/Game/Blueprints/S_CitizenSetting` (`self.CitizenSet`)))
  (bind _returnvalue (+ _citizenset_minspeed _citizenset_maxspeed))
  (set `self.CitizenSet` InCitSet)
  (set `self.Target` (`|GetArrayItem` (`self.Points`) 1))
  (set `self.Position` (`self.K2_GetActorLocation`))
  (bind _output_get (set `self.Forward` (`self.GetActorForwardVector`)))
  (set `local.StartSpeed` (/ _returnvalue 2.0))
  (set `self.Velocity` (* _output_get (/ _returnvalue 2.0))))

(fn `IsHeadingForCollision`
  (returns (NewParam :type Boolean))
  (bind (_citizenset_minspeed _citizenset_maxspeed _citizenset_maxsteerforce _citizenset_targetweight _citizenset_boundradius _citizenset_avoidcollisionweight _citizenset_collisionavoiddist) (break `/Game/Blueprints/S_CitizenSetting` (`self.CitizenSet`)))
  (bind (_position_x _position_y) (`KismetMathLibrary.BreakVector` (`self.Position`)))
  (bind (_returnvalue_x _returnvalue_y) (`KismetMathLibrary.BreakVector` (+ (* (`self.Forward`) _citizenset_collisionavoiddist) (`self.Position`))))
  (bind (_outhit _returnvalue) (`KismetSystemLibrary.SphereTraceSingleForObjects` (`KismetMathLibrary.MakeVector` _position_x _position_y) (`KismetMathLibrary.MakeVector` _returnvalue_x _returnvalue_y) _citizenset_boundradius (`|MakeArray` "ObjectTypeQuery3" :!type "EObjectTypeQuery Enum")))
  (return _returnvalue))

(fn `ObstacleRays`
  (returns (OutVector :type "Vector Structure"))
  (locals (dir :type "Vector Structure"))
  (bind (_position_x _position_y) (`KismetMathLibrary.BreakVector` (`self.Position`)))
  (bind (_citizenset_minspeed _citizenset_maxspeed _citizenset_maxsteerforce _citizenset_targetweight _citizenset_boundradius _citizenset_avoidcollisionweight _citizenset_collisionavoiddist) (break `/Game/Blueprints/S_CitizenSetting` (`self.CitizenSet`)))
  (for _array_element (`self.RDirs`)
    (bind _output_get (set `local.dir` (`KismetMathLibrary.TransformDirection` (`self.TransformCache`) _array_element)))
    (bind (_returnvalue_x _returnvalue_y) (`KismetMathLibrary.BreakVector` (+ (`self.Position`) (* _output_get _citizenset_collisionavoiddist))))
    (bind (_outhit _returnvalue) (`KismetSystemLibrary.SphereTraceSingleForObjects` (`KismetMathLibrary.MakeVector` _position_x _position_y) (`KismetMathLibrary.MakeVector` _returnvalue_x _returnvalue_y) _citizenset_boundradius (`|MakeArray` "ObjectTypeQuery3" :!type "EObjectTypeQuery Enum")))
    (if (not _returnvalue)
      (return (`local.dir`))))
  (return (`self.Forward`)))

(fn `SteerTowards`
  (params (InVector :type "Vector Structure"))
  (returns (OutVector :type "Vector Structure"))
  (locals (v :type "Vector Structure"))
  (bind (_citizenset_minspeed _citizenset_maxspeed _citizenset_maxsteerforce) (break `/Game/Blueprints/S_CitizenSetting` (`self.CitizenSet`)))
  (bind _output_get (set `local.v` (- (* (`KismetMathLibrary.Normal` InVector) _citizenset_maxspeed) (`self.Velocity`))))
  (return (`KismetMathLibrary.ClampVectorSize` _output_get 0.0 _citizenset_maxsteerforce)))

(fn `UpdateCitizen`
  (params (DT :type "Float (double-precision)"))
  (locals (TempAcceleration :type "Vector Structure") (OffsetToTarget :type "Vector Structure") (OffsetToCentre :type "Vector Structure") (collisionAvoidDir :type "Vector Structure") (collisionAvoidForce :type "Vector Structure") (speed :type "Float (double-precision)") (dir :type "Vector Structure"))
  (bind _transformcache_location (`KismetMathLibrary.BreakTransform` (`self.TransformCache`)))
  (bind _dir (`local.dir`))
  (bind (_position_x _position_y) (`KismetMathLibrary.BreakVector` (`self.Position`)))
  (bind (_citizenset_minspeed _citizenset_maxspeed _citizenset_maxsteerforce _citizenset_targetweight) (break `/Game/Blueprints/S_CitizenSetting` (`self.CitizenSet`)))
  (bind (_citizenset_minspeed_2 _citizenset_maxspeed_2 _citizenset_maxsteerforce_2 _citizenset_targetweight_2 _citizenset_boundradius _citizenset_avoidcollisionweight) (break `/Game/Blueprints/S_CitizenSetting` (`self.CitizenSet`)))
  (bind (_citizenset_minspeed_3 _citizenset_maxspeed_3) (break `/Game/Blueprints/S_CitizenSetting` (`self.CitizenSet`)))
  (bind _returnvalue (+ _transformcache_location (`self.Velocity`)))
  (set `local.TempAcceleration` (0.0 0.0 0.0))
  (`/Engine/EditorBlueprintResources/StandardMacros.IsValid` (`self.Target`)
    (:`Is Valid`
      (bind _output_get (set `local.OffsetToTarget` (- (`self.K2_GetActorLocation` (`self.Target`)) (`self.K2_GetActorLocation`))))
      (set `local.TempAcceleration` (* (`self.SteerTowards` _output_get) _citizenset_targetweight))
      (if (`self.IsHeadingForCollision`)
        (bind _output_get_2 (set `local.collisionAvoidDir` (`self.ObstacleRays`)))
        (bind _output_get_3 (set `local.collisionAvoidForce` (* (`self.SteerTowards` _output_get_2) _citizenset_avoidcollisionweight)))
        (bind _output_get_4 (set `local.TempAcceleration` (+ _output_get_3 (`local.TempAcceleration`)))))
      (bind _output_get_5 (set `self.Velocity` (+ _output_get_4 (`self.Velocity`))))
      (bind _output_get_6 (set `local.speed` (`KismetMathLibrary.VSize` _output_get_5)))
      (bind _output_get_7 (set `local.dir` (/ _output_get_5 _output_get_6)))
      (bind _output_get_8 (set `local.speed` (`KismetMathLibrary.FClamp` _output_get_6 _citizenset_minspeed_3 _citizenset_maxspeed_3)))
      (set `self.Velocity` (* _output_get_7 _output_get_8))
      (set `self.TransformCache` (`KismetMathLibrary.MakeTransform` _returnvalue))
      (set `self.CachedForward` _dir)
      (set `self.Position` _returnvalue)
      (set `self.Forward` _dir)
      (`self.K2_SetActorLocation` (`KismetMathLibrary.MakeVector` _position_x _position_y))
      (`self.K2_SetActorRotation` (`KismetMathLibrary.FindLookAtRotation` (`self.K2_GetActorLocation`) (`self.K2_GetActorLocation` (`self.Target`)))))))

(fn `UserConstructionScript`)