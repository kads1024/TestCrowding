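; Player controller for a crowd demo that places draggable path points and spawns citizens that receive them.
; Left clicks on empty space place points until two exist, then spawn a citizen at the first point and initialize it with the point list.
; Pressing on a point grabs it, and Tick moves it along XY under the cursor until release.
; A separate event starts a looping timer for repeated spawning at a clamped interval.
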(event `SpawnCharacter`
  (bind _returnvalue (`|SpawnActorFromClass` "/Game/Blueprints/BPA_Citizen.BPA_Citizen_C" (`KismetMathLibrary.MakeTransform` (`self.K2_GetActorLocation` (`|GetArrayItem` (`self.Points`)))) "Undefined" "OverrideRootScale" null null))
  (set `/Game/Blueprints/BPA_Citizen.Points` (`self.Points`) _returnvalue)
  (`/Game/Blueprints/BPA_Citizen.Initialize` :`self` _returnvalue))

(event `SpawnCharacterAtInterval`
  (params (Interval :type "Float (double-precision)"))
  (bind _returnvalue (`KismetSystemLibrary.K2_SetTimerDelegate` (delegate `SpawnCharacter`) (`KismetMathLibrary.FClamp` Interval 0.0 10.0) true))
  (set `self.SpawnHandler` _returnvalue))

(event `Key|LeftMouseButton`
  (params (Key :type "Key Structure"))
  (bind _hitresult (`self.GetHitResultUnderCursorByChannel` "TraceTypeQuery1"))
  (:`Pressed`
    (if (== (`GameplayStatics.GetObjectClass` (`.HitActor` (`GameplayStatics.BreakHitResult` _hitresult))) "/Game/Blueprints/BPA_Point.BPA_Point_C")
      (set `self.HoldingPoint` true)
      (set `self.HoldingActor` (`.HitActor` (`GameplayStatics.BreakHitResult` _hitresult)))
      (elif (>= (`KismetArrayLibrary.Array_Length` (`self.Points`)) 2)
        (`self.SpawnCharacter`)
        (else
          (bind _output_get (set `self.Location` (`.Location` (`GameplayStatics.BreakHitResult` _hitresult))))
          (bind _returnvalue (`|SpawnActorFromClass` "/Game/Blueprints/BPA_Point.BPA_Point_C" (`KismetMathLibrary.MakeTransform` (`KismetMathLibrary.MakeVector` (.x _output_get) (.y _output_get))) "Undefined" "OverrideRootScale" null null))
          (`KismetArrayLibrary.Array_Add` (`self.Points`) _returnvalue)))))
  (:`Released`
    (set `self.HoldingPoint` false)
    (set `self.HoldingActor` null)))

(event `self.ReceiveTick`
  (params (DeltaSeconds :type "Float (single-precision)"))
  (bind _hitresult (`self.GetHitResultUnderCursorByChannel` "TraceTypeQuery1"))
  (if (`self.HoldingPoint`)
    (`self.K2_SetActorLocation` (`self.HoldingActor`) (`KismetMathLibrary.MakeVector` (.x (`.Location` (`GameplayStatics.BreakHitResult` _hitresult))) (.y (`.Location` (`GameplayStatics.BreakHitResult` _hitresult)))) false false)))

(fn `UserConstructionScript`)